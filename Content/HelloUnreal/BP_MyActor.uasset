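; BP_MyActor is a practice actor whose StaticMesh shuttles back and forth along relative X.
; While IsPlay is true, Tick steps the position by a fixed, frame-rate-dependent amount, flipping IsMoveRight past either limit.
; BeginPlay runs one rightward step through the branch that Tick reuses.
; Nothing here sets IsPlay; the overlap event is empty, and debug print and delay nodes are disconnected.
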(event `self.ReceiveBeginPlay`
  ;[1 0.574 0.3047] 액터의 위치변경(x위치 변경)
  (bind _output_get (set `self.X위치` (+ (`self.X위치`) 1.0) :!label _label))
  (`SceneComponent.K2_SetRelativeLocation` (`self.StaticMesh`) (`KismetMathLibrary.MakeVector` _output_get) false false)
  (if (> (`self.X위치`) 100.0)
    (set `self.IsMoveRight` false)))

(event `self.StaticMesh.OnComponentBeginOverlap`
  (params (OverlappedComponent :type "PrimitiveComponent Object Reference") (OtherActor :type "Actor Object Reference") (OtherComp :type "PrimitiveComponent Object Reference") (OtherBodyIndex :type Integer) (bFromSweep :type Boolean) (SweepResult :type "HitResult Structure (by ref)"))
  ;[1 1 1] 뷰포트 이벤트에서 눌러서 바로 가져옴
)

(event `self.ReceiveTick`
  (params (DeltaSeconds :type "Float (single-precision)"))
  ;[1 1 1] 반복
  ;[1 1 1] 플레이어와 접촉시에만 움직임
  (if (`self.IsPlay`)
    ;[1 1 1] 변수 생성 True와 False두가지 (IF문)
    (if (`self.IsMoveRight`)
      (goto _label)
      (else
        ;[1 0.574 0.3047] 액터의 위치변경(x위치 변경_반대방향)
        (bind _output_get (set `self.X위치` (+ (`self.X위치`) -1.0)))
        (`SceneComponent.K2_SetRelativeLocation` (`self.StaticMesh`) (`KismetMathLibrary.MakeVector` _output_get) false false)
        (if (< (`self.X위치`) -100.0)
          (set `self.IsMoveRight` true))))))

(fn `UserConstructionScript`)